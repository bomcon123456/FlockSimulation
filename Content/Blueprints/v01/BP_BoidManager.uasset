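; Manager actor for a boids flocking simulation that spawns BP_Boid actors at random points inside a box on BeginPlay.
; Each Tick it computes the flock's global center and average velocity, then updates every boid's velocity from weighted cohesion, avoidance, alignment and bounding rules.
; Avoidance compares each boid against all others within range, bounding pushes strays back toward the spawn box, and velocity is capped at a limit.
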(event `self.ReceiveBeginPlay`
  (bind (_spawningstart_x _spawningstart_y _spawningstart_z) (`KismetMathLibrary.BreakVector` (`self.spawningStart`)))
  (bind (_spawningend_x _spawningend_y _spawningend_z) (`KismetMathLibrary.BreakVector` (`self.spawningEnd`)))
  (for _ (range (`self.numberOfBoids`))
    (bind _returnvalue (`|SpawnActorFromClass` "/Game/Blueprints/v01/BP_Boid.BP_Boid_C" (`KismetMathLibrary.MakeTransform` (`KismetMathLibrary.MakeVector` (`KismetMathLibrary.RandomFloatInRange` _spawningstart_x _spawningend_x) (`KismetMathLibrary.RandomFloatInRange` _spawningstart_y _spawningend_y) (`KismetMathLibrary.RandomFloatInRange` _spawningstart_z _spawningend_z))) "AlwaysSpawn" "OverrideRootScale" null null))
    (`KismetArrayLibrary.Array_Add` (`self.boids`) _returnvalue)))

(event `self.ReceiveTick`
  (params (DeltaSeconds :type "Float (single-precision)"))
  (set `self.centerOfMass` (`self.CalculateCentralMass`))
  (set `self.averageVelocity` (`self.CalculateAverageVel`))
  (for _array_element (`self.boids`)
    (set `/Game/Blueprints/v01/BP_Boid.Velocity` (* (+ (+ (+ (+ (`/Game/Blueprints/v01/BP_Boid.Velocity` _array_element) (* (`self.Rule1_Cohesion` _array_element) (`self.cohesionWeight`))) (* (`self.Rule2_Avoidance` _array_element) (`self.avoidWeight`))) (* (`self.Rule3_Alignment` _array_element) (`self.alignWeight`))) (* (`self.Rule4_Bounding` _array_element) (`self.boundsWeight`))) (`self.boidSpeedMultiplier`)) _array_element)
    (`self.LimitVelocity` _array_element)))

(fn `CalculateAverageVel`
  (returns (Output_Get :type "Vector Structure"))
  (locals (res :type "Vector Structure"))
  (bind _boids (`self.boids`))
  (for _array_element _boids
    (set `local.res` (+ (`/Game/Blueprints/v01/BP_Boid.Velocity` _array_element) (`local.res`))))
  (bind _output_get (set `local.res` (/ (`local.res`) (`KismetArrayLibrary.Array_Length` _boids))))
  (return _output_get))

(fn `CalculateCentralMass`
  (returns (Output_Get :type "Vector Structure"))
  (locals (res :type "Vector Structure"))
  (bind _boids (`self.boids`))
  (for _array_element _boids
    (set `local.res` (+ (`self.K2_GetActorLocation` _array_element) (`local.res`))))
  (bind _output_get (set `local.res` (/ (`local.res`) (`KismetArrayLibrary.Array_Length` _boids))))
  (return _output_get))

(fn `LimitVelocity`
  (params (Boids :type "/Game/Blueprints/v01/BP_Boid Object Reference"))
  (bind _velocity (`/Game/Blueprints/v01/BP_Boid.Velocity` Boids))
  (if (> (`KismetMathLibrary.VSize` _velocity) (`self.velocityLimit`))
    (set `/Game/Blueprints/v01/BP_Boid.Velocity` (* (`KismetMathLibrary.Normal` _velocity) (`self.velocityLimit`)) Boids)))

(fn `Rule1_Cohesion`
  (params (Boid :type "/Game/Blueprints/v01/BP_Boid Object Reference"))
  (returns (ReturnValue :type "Vector Structure"))
  (return (- (`self.centerOfMass`) (`self.K2_GetActorLocation` Boid))))

(fn `Rule2_Avoidance`
  (params (Boid :type "/Game/Blueprints/v01/BP_Boid Object Reference"))
  (returns (ReturnValue :type "Vector Structure"))
  (locals (distance :type "Float (double-precision)") (res :type "Vector Structure"))
  (for _array_element (`self.boids`)
    (if (!= _array_element Boid)
      (bind _returnvalue (- (`self.K2_GetActorLocation` _array_element) (`self.K2_GetActorLocation` Boid)))
      (set `local.distance` (`KismetMathLibrary.VSize` _returnvalue))
      (if (< (`local.distance`) (`self.avoidBoidRange`))
        (set `local.res` (- (`local.res`) _returnvalue)))))
  (return (`local.res`)))

(fn `Rule3_Alignment`
  (params (Boid :type "/Game/Blueprints/v01/BP_Boid Object Reference"))
  (returns (ReturnValue :type "Vector Structure"))
  (return (- (`self.averageVelocity`) (`/Game/Blueprints/v01/BP_Boid.Velocity` Boid))))

(fn `Rule4_Bounding`
  (params (Boid :type "/Game/Blueprints/v01/BP_Boid Object Reference"))
  (returns (ReturnValue :type "Vector Structure"))
  (locals (resX :type "Float (double-precision)") (resY :type "Float (double-precision)") (resZ :type "Float (double-precision)") (X :type "Float (double-precision)") (Y :type "Float (double-precision)") (Z :type "Float (double-precision)"))
  (bind (_returnvalue_x _returnvalue_y _returnvalue_z) (`KismetMathLibrary.BreakVector` (`self.K2_GetActorLocation` Boid)))
  (bind (_spawningstart_x _spawningstart_y _spawningstart_z) (`KismetMathLibrary.BreakVector` (`self.spawningStart`)))
  (bind (_spawningend_x _spawningend_y _spawningend_z) (`KismetMathLibrary.BreakVector` (`self.spawningEnd`)))
  (bind _spawningend_x_2 (`KismetMathLibrary.BreakVector` (`self.spawningEnd`)))
  (bind (_spawningstart_x_2 _spawningstart_y_2) (`KismetMathLibrary.BreakVector` (`self.spawningStart`)))
  (bind (_spawningend_x_3 _spawningend_y_2) (`KismetMathLibrary.BreakVector` (`self.spawningEnd`)))
  (bind _spawningstart_x_3 (`KismetMathLibrary.BreakVector` (`self.spawningStart`)))
  (set `local.X` _returnvalue_x)
  (set `local.Y` _returnvalue_y)
  (set `local.Z` _returnvalue_z)
  (if (< (`local.X`) _spawningstart_x_3)
    (set `local.resX` (`self.avoidSpawningBoundRange`))
    (elif (< _spawningend_x_2 (`local.X`))
      (set `local.resX` (* -1 (`self.avoidSpawningBoundRange`)))))
  (if (< (`local.Y`) _spawningstart_y_2)
    (set `local.resY` (`self.avoidSpawningBoundRange`))
    (elif (< _spawningend_y_2 (`local.Y`))
      (set `local.resY` (* -1 (`self.avoidSpawningBoundRange`)))))
  (if (< (`local.Z`) _spawningstart_z)
    (set `local.resZ` (`self.avoidSpawningBoundRange`))
    (elif (< _spawningend_z (`local.Z`))
      (set `local.resZ` (* -1 (`self.avoidSpawningBoundRange`)))))
  (return (`KismetMathLibrary.Normal` (`KismetMathLibrary.MakeVector` (`local.resX`) (`local.resY`) (`local.resZ`)))))

(fn `UserConstructionScript`)