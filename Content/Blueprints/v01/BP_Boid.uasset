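; BP_Boid is an early boid actor that drifts at a constant velocity, with no flocking behavior in its graphs.
; BeginPlay picks a small random velocity on each axis, and Tick applies it as an unswept local-space offset scaled by delta time.
; An unconnected node chain holds an alternative interpolated move that would also rotate the actor toward its velocity with a roll correction.
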(event `self.ReceiveBeginPlay`
  (set `self.Velocity` (`KismetMathLibrary.MakeVector` (`KismetMathLibrary.RandomFloatInRange` -5.0 5.0) (`KismetMathLibrary.RandomFloatInRange` -5.0 5.0) (`KismetMathLibrary.RandomFloatInRange` -5.0 5.0))))

(event `self.ReceiveTick`
  (params (DeltaSeconds :type "Float (single-precision)"))
  (`self.K2_AddActorLocalOffset` (* (`self.Velocity`) DeltaSeconds)))

(fn `UserConstructionScript`)